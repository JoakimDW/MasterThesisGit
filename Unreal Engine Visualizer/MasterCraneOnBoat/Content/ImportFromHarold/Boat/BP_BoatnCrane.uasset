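; Boat actor carrying a child BP_Crane, linking the crane's boom cylinder to an external TwinCAT PLC over ADS.
; Construction script binds force, velocity and position variables to the TwinCAT master and names, with force read cyclically and the others written.
; Tick pushes the hull mesh with a force, sends piston velocity and position out, and feeds cylinder force into the crane, converting units by 100.
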(event EventBeginPlay)

(event Collision|EventActorBeginOverlap
  (params (OtherActor :type Actor%20Object%20Reference)))

(event EventTick
  (params (DeltaSeconds :type Float%20%28single-precision%29))
  (Physics|AddForce (Variables|Default|Getsalt_sov_rr) (Variables|Default|GetForce) "None" false)
  (bind _asbp_crane (Utilities|Casting|CastToBP_Crane (Variables|/Script/Engine.ChildActorComponent|GetChildActor (Variables|Default|GetBP_Crane))))
  (bind _output_get (Variables|/Script/TwinCatAdsApi.TcAdsVariable|SetValue (Variables|Default|GetBoomCylVel) (/ (Variables|/Game/ImportFromHarold/Crane/BP_Crane.BP_Crane_C|GetBoomPistVel _asbp_crane) 1e+02)))
  (Variables|Default|SetBoom%20Pist%20Vel _output_get)
  (bind _output_get_2 (Variables|/Script/TwinCatAdsApi.TcAdsVariable|SetValue (Variables|Default|GetBoomCylPos) (/ (Variables|/Game/ImportFromHarold/Crane/BP_Crane.BP_Crane_C|GetBoomPistPos _asbp_crane) 1e+02)))
  (Variables|Default|SetBoom%20Pist%20Pos _output_get_2)
  (bind _output_get_3 (Variables|/Game/ImportFromHarold/Crane/BP_Crane.BP_Crane_C|SetBoomCylForce _asbp_crane (* (Variables|/Script/TwinCatAdsApi.TcAdsVariable|GetValue (Variables|Default|GetBoomCylForce)) 1e+02)))
  (Variables|Default|SetBoom%20Cyl%20Force%20Thing _output_get_3))

(fn ConstructionScript
  (bind _boomcylvel (Variables|Default|GetBoomCylVel))
  (bind _boomcylpos (Variables|Default|GetBoomCylPos))
  (bind _boomcylforce (Variables|Default|GetBoomCylForce))
  (bind _output_get (Variables|/Script/TwinCatAdsApi.TcAdsVariable|SetAdsMaster _boomcylforce (Variables|Default|GetTc%20Master)))
  (bind _output_get_2 (Variables|/Script/TwinCatAdsApi.TcAdsVariable|SetAdsMaster _boomcylvel _output_get))
  (Variables|/Script/TwinCatAdsApi.TcAdsVariable|SetAdsMaster _boomcylpos _output_get_2)
  (Variables|/Script/TwinCatAdsApi.TcAdsVariable|SetAdsName _boomcylforce (Variables|ADSnames|GetBoomCylForceName))
  (Variables|/Script/TwinCatAdsApi.TcAdsVariable|SetAdsName _boomcylvel (Variables|ADSnames|GetBoomCylVelName))
  (Variables|/Script/TwinCatAdsApi.TcAdsVariable|SetAdsName _boomcylpos (Variables|ADSnames|GetBoom%20Cyl%20Pos%20Name))
  (Variables|/Script/TwinCatAdsApi.TcAdsVariable|SetAccess _boomcylforce "ReadCyclic")
  (Variables|/Script/TwinCatAdsApi.TcAdsVariable|SetAccess _boomcylvel "Write")
  (Variables|/Script/TwinCatAdsApi.TcAdsVariable|SetAccess _boomcylpos "Write")
  (Variables|/Script/TwinCatAdsApi.TcAdsVariable|SetValue (Variables|Default|GetBoomCylForce) (Variables|Default|GetBoom%20Cyl%20Force%20Thing)))