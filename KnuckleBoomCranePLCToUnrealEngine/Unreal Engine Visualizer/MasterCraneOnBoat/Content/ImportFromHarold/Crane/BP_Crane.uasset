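; BP_Crane is a crane Blueprint that physically drives its main boom's paired hydraulic cylinders.
; Each Tick applies opposing BoomCylForce-sized forces to two piston rods and two cylinder bodies, all directed along one cylinder's X axis.
; It also measures the first piston's extension and derives its velocity through a Differentiate helper, storing both without using them in this graph.
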(event EventBeginPlay)

(event Collision|EventActorBeginOverlap
  (params (OtherActor :type Actor%20Object%20Reference)))

(event EventTick
  (params (DeltaSeconds :type Float%20%28single-precision%29))
  (bind _mainboom_cylinder_solid4 (Variables|Default|GetMainBoom_Cylinder_Solid4))
  (bind _boomcylforce (Variables|Default|GetBoomCylForce))
  (bind _returnvalue (Transformation|GetWorldRotation _mainboom_cylinder_solid4))
  (bind _returnvalue_2 (Math|Vector|MakeVector _boomcylforce 0.0 0.0))
  (bind _returnvalue_3 (Math|Vector|RotateVector _returnvalue_2 _returnvalue))
  (bind _returnvalue_4 (Math|Vector|NegateVector _returnvalue_3))
  (bind _output_get (Variables|Default|SetBoomPistPos (Math|Vector|Distance(Vector) (Transformation|GetWorldLocation (Variables|Default|GetMainBoom_PistonRod)) (Transformation|GetWorldLocation (Variables|Default|GetMainBoom_Cylinder_Solid4)))))
  (bind (_diff _value_out) (CallFunction|Differentiate _output_get DeltaSeconds (Variables|Default|GetPrevBoomPistPos)))
  (Variables|Default|SetPrevBoomPistPos _value_out)
  (Variables|Default|SetBoomPistVel _diff)
  (Physics|AddForce (Variables|Default|GetMainBoom_PistonRod) _returnvalue_3 "None" false)
  (Physics|AddForce _mainboom_cylinder_solid4 _returnvalue_4 "None" false)
  (Physics|AddForce (Variables|Default|GetMainBoom_Cylinder_Solid5) _returnvalue_4 "None" false)
  (Physics|AddForce (Variables|Default|GetMainBoom_PistonRod1) _returnvalue_3 "None" false))

(fn ConstructionScript)

(fn Differentiate
  (params (Value%20In :type Float%20%28single-precision%29) (DeltaTime :type Float%20%28single-precision%29) (PrevValue :type Float%20%28single-precision%29))
  (return (/ (- Value%20In PrevValue) DeltaTime) Value%20In))